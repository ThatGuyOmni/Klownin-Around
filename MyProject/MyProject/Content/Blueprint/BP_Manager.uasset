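; BP_Manager runs a repeating round cycle that alternates timed AI spawning phases with evacuation phases.
; On BeginPlay it activates each valid referenced spawner and has it spawn AI, then starts a one-minute timer.
; When that expires it enables the evac flag and deactivates the spawners, and a second one-minute timer clears the flag and restarts the round.
; Both timers are set inside the spawner loops, so they require a valid spawner.
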(event Custom|Round%20Start
  (for _array_element (Variables|Default|GetSpawnerReference)
    (Utilities|IsValid _array_element
      (:Is%20Valid
        (Default|SpawnerActive _array_element)
        (Default|SpawnAI _array_element)
        (Utilities|Time|SetTimerbyEvent (delegate Custom|Round) 6e+01)))))

(event Custom|Round
  (CallFunction|Evac)
  (for _array_element (Variables|Default|GetSpawnerReference)
    (Utilities|IsValid _array_element
      (:Is%20Valid
        (Default|SpawnerInactive _array_element)
        (Utilities|Time|SetTimerbyEvent (delegate Custom|New%20Round) 6e+01))
      (:Is%20Not%20Valid
        (Development|PrintString "Second Node")))))

(event Custom|Evac
  (Variables|/Game/Blueprint/BP_EvacPoint.BP_EvacPoint_C|SetEvac%20On (Variables|Default|GetEvacReference) true))

(event Custom|New%20Round
  (Variables|/Game/Blueprint/BP_EvacPoint.BP_EvacPoint_C|SetEvac%20On (Variables|Default|GetEvacReference) false)
  (CallFunction|RoundStart))

(event EventBeginPlay
  (CallFunction|RoundStart))

(fn ConstructionScript)
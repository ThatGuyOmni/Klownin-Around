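; BP_Spawner is a switchable spawner that repeatedly spawns an AI actor at its own location while it is on.
; SpawnerActive and SpawnerInactive only set the SpawnerOn flag; SpawnAI checks it and starts a one-shot timer of SpawnTimer length.
; When the timer fires, SpawnLoop spawns the SpawnedAI class and calls SpawnAI again, so the cycle repeats until the flag is off at the next check.
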(event Custom|Spawn%20AI
  (if (Variables|Default|GetSpawnerOn)
    (Utilities|Time|SetTimerbyEvent (delegate Custom|SpawnLoop) (Variables|Default|GetSpawnTimer))))

(event Custom|SpawnerActive
  ;[0 1 0.1846] Turn On Spawner
  (Variables|Default|SetSpawnerOn true))

(event Custom|SpawnLoop
  (Game|SpawnActorfromClass (Variables|Default|GetSpawned%20AI) (Math|Transform|MakeTransform (Transformation|GetActorLocation) "0, 0, 0" "1.000000,1.000000,1.000000") "Undefined" "MultiplyWithRoot" 0 0)
  (CallFunction|SpawnAI))

(event Custom|SpawnerInactive
  ;[1 0 0.06069] Turn Off Spawner
  (Variables|Default|SetSpawnerOn false))

(fn ConstructionScript)
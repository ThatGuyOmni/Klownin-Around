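; Behavior tree task that makes an AI pawn attack its blackboard Target by firing a clown missile.
; When CanFire is set, it spawns BP_ClownMissile offset from the pawn and rotated toward the target, then clears the flag.
; The cooldown length comes from the BP_Stun actor found in the level.
; After that delay, it re-enables firing and finishes successfully, with debug prints along the way.
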(event EventReceiveExecuteAI
  (params (OwnerController :type AI%20Controller%20Object%20Reference) (ControlledPawn :type Pawn%20Object%20Reference))
  (bind _returnvalue (Transformation|GetActorLocation ControlledPawn))
  (Development|PrintString (Utilities|String|ToString(Boolean) (Variables|Default|GetCanFire?)))
  (if (Variables|Default|GetCanFire?)
    (Development|PrintString "Attack")
    (Game|SpawnActorfromClass "/Game/Blueprints/BP_ClownMissile.BP_ClownMissile_C" (Math|Transform|MakeTransform (+ _returnvalue "80.000000,0.000000,30.000000") (Math|Rotator|FindLookatRotation _returnvalue (Transformation|GetActorLocation (.AsActor (Utilities|Casting|CastToActor (AI|Components|Blackboard|GetValueasObject (Variables|/Script/AIModule.AIController|GetBlackboard OwnerController) (Utilities|Name|MakeLiteralName "Target")))))) "1.000000,1.000000,1.000000") "Undefined" "MultiplyWithRoot" 0 0)
    (Variables|Default|SetCanFire? false)
    (Development|PrintString "Cooldwn")
    (bind _returnvalue_2 (Actor|GetActorOfClass "/Game/Blueprints/BP_Stun.BP_Stun_C"))
    (bind _output_get (Variables|Default|SetManager _returnvalue_2))
    (Development|PrintString (Utilities|String|ToString(Float) (Variables|/Game/Blueprints/BP_Stun.BP_Stun_C|GetWaitLength _output_get))))
  (Utilities|FlowControl|Delay (Variables|/Game/Blueprints/BP_Stun.BP_Stun_C|GetWaitLength _output_get))
  (Variables|Default|SetCanFire? true)
  (AI|BehaviorTree|FinishExecute true))
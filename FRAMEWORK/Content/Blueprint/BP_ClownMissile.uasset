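; BP_ClownMissile is a clown missile actor that kills sports car pawns on contact.
; When its sphere overlaps an actor, it calls Dead on a SportsCar_Pawn, sends DestroyMessage to whatever it hit, then destroys itself.
; A timer started at BeginPlay removes the missile if nothing is hit.
; Its Is Human and Is Klown queries both return false, identifying it as neither side.
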(event OnComponentBeginOverlap(Sphere)
  (params (OverlappedComponent :type Primitive%20Component%20Object%20Reference) (OtherActor :type Actor%20Object%20Reference) (OtherComp :type Primitive%20Component%20Object%20Reference) (OtherBodyIndex :type Integer) (bFromSweep :type Boolean) (SweepResult :type Hit%20Result%20Structure%20%28by%20ref%29))
  (bind _assports_car_pawn (Utilities|Casting|CastToSportsCar_Pawn OtherActor)
    (:then
      (Default|Dead _assports_car_pawn))
    (:CastFailed
      _))
  (Class|BPIKlownStuff|Destroy(Message) OtherActor)
  (Actor|DestroyActor))

(event EventBeginPlay
  (Utilities|FlowControl|Delay 1e+01)
  (Actor|DestroyActor))

(fn ConstructionScript)

(fn IsHuman?
  (return false))

(fn IsKlown?
  (return false))
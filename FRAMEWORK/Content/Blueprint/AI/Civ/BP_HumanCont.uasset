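; AI controller for human civilians that runs the BT_Human behavior tree and tracks Klown threats through AI perception.
; A perceived actor that identifies as a Klown is written to the KlownThreat blackboard key.
; When the stimulus is lost, a visibility trace from the pawn clears the key only if it does not hit that Klown, so threats in line of sight persist.
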(event OnTargetPerceptionUpdated(AIPerception)
  (params (Actor :type Actor%20Object%20Reference) (Stimulus :type AI%20Stimulus%20Structure))
  (bind _klown_ (Class|BPIKlownStuff|IsKlown?(Message) Actor))
  (if _klown_
    (if (.bSuccessfullySensed (Utilities|Struct|BreakAIStimulus Stimulus))
      (AI|Components|Blackboard|SetValueasObject (AI|GetBlackboard 0) (Utilities|Name|MakeLiteralName "KlownThreat") Actor)
      (else
        (bind _outhit (Collision|LineTraceByChannel (Transformation|GetActorLocation (Pawn|GetControlledPawn)) (Transformation|GetActorLocation Actor) "TraceTypeQuery1" false 0 "None"))
        (if (not (== Actor (.HitActor (Collision|BreakHitResult _outhit))))
          (AI|Components|Blackboard|SetValueasObject (AI|GetBlackboard 0) (Utilities|Name|MakeLiteralName "KlownThreat") 0))))))

(event EventBeginPlay
  (AI|RunBehaviorTree "/Game/Blueprint/AI/Civ/BT_Human.BT_Human"))

(fn ConstructionScript)
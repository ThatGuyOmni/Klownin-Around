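; BP_CivCont is an AI controller for civilian characters, running the BT_Civ behavior tree on BeginPlay.
; Its AIPerception update writes a successfully sensed actor to the Target blackboard key and clears that key when an update reports the sensing failed.
; Debug prints announce startup and each spotted or lost actor.
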(event OnTargetPerceptionUpdated(AIPerception)
  (params (Actor :type Actor%20Object%20Reference) (Stimulus :type AI%20Stimulus%20Structure))
  (bind _returnvalue (Utilities|GetDisplayName Actor))
  (bind _returnvalue_2 (AI|GetBlackboard 0))
  (bind _returnvalue_3 (Utilities|Name|MakeLiteralName "Target"))
  (if (.bSuccessfullySensed (Utilities|Struct|BreakAIStimulus Stimulus))
    (Development|PrintString (Utilities|String|Append "Spotted " _returnvalue) true true "(R=0.000000,G=0.054793,B=1.000000,A=1.000000)")
    (AI|Components|Blackboard|SetValueasObject _returnvalue_2 _returnvalue_3 Actor)
    (else
      (Development|PrintString (Utilities|String|Append "Lost sight of" _returnvalue) true true "(R=1.000000,G=0.000000,B=0.036017,A=1.000000)")
      (AI|Components|Blackboard|SetValueasObject _returnvalue_2 _returnvalue_3 0))))

(event EventBeginPlay
  (AI|RunBehaviorTree "/Game/Blueprints/AI/Civ/BT_Civ.BT_Civ")
  (Development|PrintString "Hello"))

(fn ConstructionScript)
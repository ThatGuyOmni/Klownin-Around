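; Round manager that alternates timed spawning and evacuation phases and creates the game UI.
; It gathers every BP_Spawner, runs them for a minute, then deactivates them while the evac, player waypoint and UI countdown run for another minute.
; Each new round raises Clownification, dividing spawn timers by it and enlarging existing BP_Klown actors.
; PlusOne counts collected people and calls CallNewRescue.
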(event Custom|Round%20Start
  (Development|PrintString (Utilities|String|Append "Round Number: " (Utilities|String|ToString(Integer) (Variables|Default|GetClownification))))
  (for _array_element (Variables|Default|GetSpawnerReference)
    (Utilities|IsValid _array_element
      (:Is%20Valid
        (Default|SpawnerActive _array_element)
        (Default|SpawnAI _array_element)
        (Utilities|Time|SetTimerbyEvent (delegate Custom|Round) 6e+01)))))

(event Custom|Round
  (Default|EvacActive (Variables|Default|GetEvacReference))
  (Default|ActivateWayPoint (Variables|Default|GetPlayerRef))
  (for _array_element (Variables|Default|GetSpawnerReference)
    (Utilities|IsValid _array_element
      (:Is%20Valid
        (Default|SpawnerInactive _array_element)
        ;[1 1 1] During the second half of the round the player cannot drop off any civs
        (Default|CountdownTillEvacLeaves (stale EventBeginPlay _returnvalue))
        (Utilities|Time|SetTimerbyEvent (delegate Custom|New%20Round) 6e+01))
      (:Is%20Not%20Valid
        (Development|PrintString "Second Node")))))

(event Custom|PlusOne
  (Math|Integer|IncrementInt (Variables|Default|GetPeopleCollected)
    (:%20%20
      (Default|CallNewRescue))))

(event Custom|New%20Round
  ;[1 1 1] During the second half of the round the player cannot drop off any civs
  (Default|EvacDeactive (Variables|Default|GetEvacReference))
  (Math|Integer|IncrementInt (Variables|Default|GetClownification)
    (:%20%20
      (CallFunction|Clownify)
      (CallFunction|RoundStart))))

(event EventBeginPlay
  (CallFunction|InitSpawners)
  (Variables|Default|SetClownification 1)
  (CallFunction|RoundStart)
  (bind _returnvalue (UserInterface|CreateWidget "/Game/UI/GameUI.GameUI_C"))
  (UserInterface|Viewport|AddtoViewport _returnvalue 0))

(fn ConstructionScript)

(fn Clownify
  (for _array_element (Variables|Default|GetSpawnerReference)
    (Variables|/Game/Blueprint/Spawners_And_Managers/BP_Spawner.BP_Spawner_C|SetSpawnTimer _array_element (/ (Variables|/Game/Blueprint/Spawners_And_Managers/BP_Spawner.BP_Spawner_C|GetSpawnTimer _array_element) (Variables|Default|GetClownification))))
  (bind _outactors (Actor|GetAllActorsOfClass "/Game/Blueprint/AI/Klown/BP_Klown.BP_Klown_C"))
  (for _array_element_2 _outactors
    (Transformation|SetActorScale3D _array_element_2 (* (Transformation|GetActorScale3D _array_element_2) 1.5))))

(fn InitSpawners
  (bind _outactors (Actor|GetAllActorsOfClass "/Game/Blueprint/Spawners_And_Managers/BP_Spawner.BP_Spawner_C"))
  (for _array_element _outactors
    (Utilities|Array|Add (Variables|Default|GetSpawnerReference) _array_element)))
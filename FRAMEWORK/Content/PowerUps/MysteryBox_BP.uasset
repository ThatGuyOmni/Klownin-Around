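; Mystery box pickup that gives an overlapping SportsCar_Pawn a power-up, then hides and disables its collision for ten seconds before respawning.
; A timeline started on BeginPlay bobs the actor vertically from its start location.
; The power-up switch has a fixed input of 0, so it always grants the first enum value; the random-integer node is unused.
; The cube's spin timeline is never run.
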(event OnComponentBeginOverlap(Box)
  (params (OverlappedComponent :type Primitive%20Component%20Object%20Reference) (OtherActor :type Actor%20Object%20Reference) (OtherComp :type Primitive%20Component%20Object%20Reference) (OtherBodyIndex :type Integer) (bFromSweep :type Boolean) (SweepResult :type Hit%20Result%20Structure%20%28by%20ref%29))
  (bind _assports_car_pawn (Utilities|Casting|CastToSportsCar_Pawn OtherActor))
  (switch int 0
    (:0
      (Variables|Default|SetpowerUps "NewEnumerator0"))
    (:1
      (Variables|Default|SetpowerUps "NewEnumerator1"))
    (:2
      (Variables|Default|SetpowerUps "NewEnumerator2")))
  (Default|SetPowerUp _assports_car_pawn (Variables|Default|GetpowerUps))
  (Collision|SetCollisionEnabled (Variables|Default|GetBox) "NoCollision")
  (Rendering|SetVisibility (Variables|Default|GetCube) false false)
  (Utilities|FlowControl|Delay 1e+01)
  (Collision|SetCollisionEnabled (Variables|Default|GetBox) "QueryAndPhysics")
  (Rendering|SetVisibility (Variables|Default|GetCube) true false))

(event Custom|Movement
  (bind _startlocation (Variables|Default|GetStartLocation))
  ;[1 1 1] Movement
  (Utilities|FlowControl|Sequence
    (:then_0
      (bind _newtrack_0 (Timeline|Upanddown Play)
        (:Update
          (Transformation|SetActorLocation (Math|Vector|Lerp(Vector) _startlocation (+ _startlocation "0.000000,0.000000,30.000000") _newtrack_0) false false))))))

(event EventBeginPlay
  ;[1 1 1] Movement
  (Variables|Default|SetStartLocation (Transformation|GetActorLocation))
  (Variables|Default|SetStartRotator (Variables|/Script/Engine.SceneComponent|GetRelativeRotation (Variables|Default|GetCube)))
  (CallFunction|Movement))

(fn ConstructionScript)
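; AI controller for Klown characters that runs the BT_Klown behavior tree on begin play.
; AI perception updates filter for human actors and write a sensed one to the Blackboard's Target key.
; When perception loses a human, a visibility trace from the pawn to that actor clears Target only if it fails to hit them.
; Its own IsHuman and IsKlown checks both return false.
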(event OnTargetPerceptionUpdated(AIPerception)
  (params (Actor :type Actor%20Object%20Reference) (Stimulus :type AI%20Stimulus%20Structure))
  (bind _returnvalue (AI|GetBlackboard 0))
  (bind _returnvalue_2 (Utilities|Name|MakeLiteralName "Target"))
  (bind _human_ (Class|BPIKlownStuff|IsHuman?(Message) Actor))
  (if _human_
    (if (.bSuccessfullySensed (Utilities|Struct|BreakAIStimulus Stimulus))
      (AI|Components|Blackboard|SetValueasObject _returnvalue _returnvalue_2 Actor)
      (else
        (bind _outhit (Collision|LineTraceByChannel (Transformation|GetActorLocation (Pawn|GetControlledPawn)) (Transformation|GetActorLocation Actor) "TraceTypeQuery1" false 0 "None"))
        (if (not (== Actor (.HitActor (Collision|BreakHitResult _outhit))))
          (AI|Components|Blackboard|SetValueasObject _returnvalue _returnvalue_2 0))))))

(event EventBeginPlay
  (AI|RunBehaviorTree "/Game/Blueprint/AI/Klown/BT_Klown.BT_Klown"))

(fn ConstructionScript)

(fn IsHuman?
  (return false))

(fn IsKlown?
  (return false))
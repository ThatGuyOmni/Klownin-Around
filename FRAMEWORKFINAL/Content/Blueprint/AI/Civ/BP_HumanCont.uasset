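; AI controller for human civilians that runs the BT_Human behavior tree and feeds it what the pawn perceives.
; Perception updates set the KlownThreat blackboard key for klowns, identified by an IsKlownMessage call, and the Target key for sports car pawns.
; Losing a car clears Target immediately, while losing a klown clears KlownThreat only if a visibility trace from the pawn fails to hit it.
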(event OnTargetPerceptionUpdated(AIPerception)
  (params (Actor :type Actor%20Object%20Reference) (Stimulus :type AI%20Stimulus%20Structure))
  (bind _bsuccessfullysensed (Utilities|Struct|BreakAIStimulus Stimulus))
  (bind _returnvalue (AI|GetBlackboard 0))
  (bind _returnvalue_2 (Utilities|Name|MakeLiteralName "Target"))
  (bind _klown_ (Class|BPIKlownStuff|IsKlown?(Message) Actor))
  (if _klown_
    (if _bsuccessfullysensed
      (AI|Components|Blackboard|SetValueasObject (AI|GetBlackboard 0) (Utilities|Name|MakeLiteralName "KlownThreat") Actor)
      (else
        (bind _outhit (Collision|LineTraceByChannel (Transformation|GetActorLocation (Pawn|GetControlledPawn)) (Transformation|GetActorLocation Actor) "TraceTypeQuery1" false 0 "None"))
        (if (not (== Actor (.HitActor (Collision|BreakHitResult _outhit))))
          (AI|Components|Blackboard|SetValueasObject (AI|GetBlackboard 0) (Utilities|Name|MakeLiteralName "KlownThreat") 0))))
    (else
      (bind _assports_car_pawn (Utilities|Casting|CastToSportsCar_Pawn Actor))
      (if _bsuccessfullysensed
        (AI|Components|Blackboard|SetValueasObject _returnvalue _returnvalue_2 _assports_car_pawn)
        (else
          (AI|Components|Blackboard|SetValueasObject _returnvalue _returnvalue_2 0))))))

(event EventBeginPlay
  (AI|RunBehaviorTree "/Game/Blueprint/AI/Civ/BT_Human.BT_Human"))

(fn ConstructionScript)
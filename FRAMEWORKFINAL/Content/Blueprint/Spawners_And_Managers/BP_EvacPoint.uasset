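; BP_EvacPoint is an evacuation zone that reports to a manager when the player's sports car drives into it while active.
; EvacActive and EvacDeactive events toggle the EvacOn flag and the Area component's visibility, which the construction script hides by default.
; Collision overlaps from SportsCar_Pawn call UpdateRescued on ManagerRef with zero, only while EvacOn is true.
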(event OnComponentBeginOverlap(Collision)
  (params (OverlappedComponent :type Primitive%20Component%20Object%20Reference) (OtherActor :type Actor%20Object%20Reference) (OtherComp :type Primitive%20Component%20Object%20Reference) (OtherBodyIndex :type Integer) (bFromSweep :type Boolean) (SweepResult :type Hit%20Result%20Structure%20%28by%20ref%29))
  (Utilities|Casting|CastToSportsCar_Pawn OtherActor)
  (if (Variables|Default|GetEvac%20On)
    (Default|UpdateRescued (Variables|Default|GetManagerRef))))

(event Custom|EvacActive
  (bind _output_get (Variables|Default|SetEvac%20On true))
  (Rendering|SetVisibility (Variables|Default|Getarea) _output_get false)
  (Development|PrintString "evac appear"))

(event Custom|EvacDeactive
  (bind _output_get (Variables|Default|SetEvac%20On false))
  (Rendering|SetVisibility (Variables|Default|Getarea) _output_get false))

(fn ConstructionScript
  (Rendering|SetVisibility (Variables|Default|Getarea) false false))
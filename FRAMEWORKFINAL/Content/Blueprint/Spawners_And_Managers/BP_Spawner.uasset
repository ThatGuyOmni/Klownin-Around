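; BP_Spawner repeatedly spawns an AI actor at random points in a large square around itself, at a fixed world height.
; SpawnerActive and SpawnerInactive set a flag that SpawnAI checks before starting a one-shot timer of SpawnTimer length.
; The timer spawns SpawnedAI and calls SpawnAI again to re-arm.
; Turning the flag on does not itself start the loop.
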(event Custom|Spawn%20AI
  (if (Variables|Default|GetSpawnerOn)
    (Utilities|Time|SetTimerbyEvent (delegate Custom|SpawnLoop) (Variables|Default|GetSpawnTimer))))

(event Custom|SpawnerActive
  ;[0 1 0.1846] Turn On Spawner
  (Variables|Default|SetSpawnerOn true))

(event Custom|SpawnLoop
  (bind _returnvalue (Transformation|GetActorLocation))
  (Game|SpawnActorfromClass (Variables|Default|GetSpawned%20AI) (Math|Transform|MakeTransform (Math|Vector|MakeVector (+ (Math|Random|RandomFloatinRange -2e+04 2e+04) (.x _returnvalue)) (+ (Math|Random|RandomFloatinRange -2e+04 2e+04) (.y _returnvalue)) 3e+01) "0, 0, 0" "1.000000,1.000000,1.000000") "Undefined" "OverrideRootScale" 0 0)
  (CallFunction|SpawnAI))

(event Custom|SpawnerInactive
  ;[1 0 0.06069] Turn Off Spawner
  (Variables|Default|SetSpawnerOn false))

(fn ConstructionScript)
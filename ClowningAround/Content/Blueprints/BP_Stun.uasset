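; BP_Stun is an unfinished pickup actor, apparently for a stun ability in a top-down game.
; When a BP_TopDownCharacter overlaps its sphere, it caches that player, hides its components and sets a wait length that is not read here.
; Pressing F runs a multi-sphere trace from the player's mesh and prints a debug string.
; The trace results are unused, so no stun is applied.
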(event OnComponentBeginOverlap(Sphere)
  (params (OverlappedComponent :type Primitive%20Component%20Object%20Reference) (OtherActor :type Actor%20Object%20Reference) (OtherComp :type Primitive%20Component%20Object%20Reference) (OtherBodyIndex :type Integer) (bFromSweep :type Boolean) (SweepResult :type Hit%20Result%20Structure%20%28by%20ref%29))
  (bind _asbp_top_down_character (Utilities|Casting|CastToBP_TopDownCharacter OtherActor))
  (Variables|Default|Setplayer _asbp_top_down_character)
  (Rendering|SetVisibility (Variables|Default|GetDefaultSceneRoot) false true)
  (Variables|Default|SetWaitLength 1e+01))

(event EventBeginPlay)

(event Collision|EventActorBeginOverlap
  (params (OtherActor :type Actor%20Object%20Reference)))

(event EventTick
  (params (DeltaSeconds :type Float%20%28single-precision%29)))

(event Input|KeyboardEvents|F
  (params (Key :type Key%20Structure :default "None"))
  (:Pressed
    (Collision|MultiSphereTraceByChannel (Transformation|GetWorldLocation (Variables|/Script/Engine.Character|GetMesh (Variables|Default|Getplayer))) "0, 0, 0" 0.0 "TraceTypeQuery1" false 0 "None")
    (Development|PrintString "woah")))

(fn ConstructionScript)